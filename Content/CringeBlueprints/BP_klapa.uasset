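; BP_klapa is an interactable actor, apparently a flap or hatch, that rotates its static mesh on interaction.
; The BPI_interactklapa event is gated by IsOpening and uses a FlipFlop to alternate between playing a Timeline and reversing it from the end.
; Timeline updates clear IsOpening and set the mesh's relative rotation to a fixed value, with no interpolation shown.
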(event `BPI_interactklapa`
  (if (not (`self.IsOpening`))
    (for _ (`|MakeArray` (`self.StaticMesh`))
      (`/Engine/EditorBlueprintResources/StandardMacros.FlipFlop`
        (:`A`
          (set `self.IsOpening` true)
          (`Timeline|Timeline` :!label _label
            (:`Update`
              (set `self.IsOpening` false)
              (`SceneComponent.K2_SetRelativeRotation` (`self.StaticMesh`) (struct :`Pitch` 100.0) false false))))
        (:`B`
          (set `self.IsOpening` true)
          (goto _label :!via `ReverseFromEnd`))))))

(fn `UserConstructionScript`)