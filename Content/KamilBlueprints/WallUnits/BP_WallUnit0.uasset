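; Interactive wall unit whose thirteen box components swing open and closed by 90 degrees when the player interacts with them.
; BPI_CheckComponent stores the targeted component and picks its rotation axis and direction from hardcoded component groups.
; BPI_PlayerInteract uses a FlipFlop per component to play or reverse one shared Timeline that lerps relative rotation.
; Flags block retargeting and further interaction until the animation finishes, so one part moves at a time.
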(event `BPI_PlayerInteract_1`
  (if (not (`self.IsOpening`))
    (for (_array_element _array_index) (`|MakeArray` (`self.box_2_pol_2`) (`self.box_1_typ_13`) (`self.box_4_pol_8`) (`self.box_4_pol_7`) (`self.box_4_pol_5`) (`self.box_4_pol_6`) (`self.box_5_pol_2`) (`self.box_4_pol_3`) (`self.box_4_pol_4`) (`self.box_4_pol_2`) (`self.box_4_pol_1`) (`self.box_6_pol_2`) (`self.box_6_pol_1`))
      (if (== _array_element (`self.TargetComponent`))
        (switch `int` _array_index
          (:`0`
            (`/Engine/EditorBlueprintResources/StandardMacros.FlipFlop`
              (:`A`
                (set `self.CanSetTarget` false :!label _label)
                (set `self.IsOpening` true)
                (bind (_direction _newtrack_0) (`Timeline|Timeline` :!via `PlayFromStart` :!label _label_2)
                  (:`Update`
                    (`SceneComponent.K2_SetRelativeRotation` (`self.TargetComponent`) (`KismetMathLibrary.RLerp` (struct) (select `int` (`self.RotationIndex`) :`0` (struct :`Pitch` 90.0) :`1` (struct :`Pitch` -90.0) :`2` (struct :`Roll` 90.0) :!type "Rotator Structure") _newtrack_0) false false))
                  (:`Finished`
                    (set `self.CanSetTarget` true)
                    (set `self.IsOpening` false))))
              (:`B`
                (set `self.CanSetTarget` false :!label _label_3)
                (set `self.IsOpening` true)
                (goto _label_2 :!via `ReverseFromEnd`))))
          (:`1`
            (`/Engine/EditorBlueprintResources/StandardMacros.FlipFlop`
              (:`A`
                (goto _label))
              (:`B`
                (goto _label_3))))
          (:`2`
            (`/Engine/EditorBlueprintResources/StandardMacros.FlipFlop`
              (:`A`
                (goto _label))
              (:`B`
                (goto _label_3))))
          (:`3`
            (`/Engine/EditorBlueprintResources/StandardMacros.FlipFlop`
              (:`A`
                (goto _label))
              (:`B`
                (goto _label_3))))
          (:`4`
            (`/Engine/EditorBlueprintResources/StandardMacros.FlipFlop`
              (:`A`
                (goto _label))
              (:`B`
                (goto _label_3))))
          (:`5`
            (`/Engine/EditorBlueprintResources/StandardMacros.FlipFlop`
              (:`A`
                (goto _label))
              (:`B`
                (goto _label_3))))
          (:`6`
            (`/Engine/EditorBlueprintResources/StandardMacros.FlipFlop`
              (:`A`
                (goto _label))
              (:`B`
                (goto _label_3))))
          (:`7`
            (`/Engine/EditorBlueprintResources/StandardMacros.FlipFlop`
              (:`A`
                (goto _label))
              (:`B`
                (goto _label_3))))
          (:`8`
            (`/Engine/EditorBlueprintResources/StandardMacros.FlipFlop`
              (:`A`
                (goto _label))
              (:`B`
                (goto _label_3))))
          (:`9`
            (`/Engine/EditorBlueprintResources/StandardMacros.FlipFlop`
              (:`A`
                (goto _label))
              (:`B`
                (goto _label_3))))
          (:`10`
            (`/Engine/EditorBlueprintResources/StandardMacros.FlipFlop`
              (:`A`
                (goto _label))
              (:`B`
                (goto _label_3))))
          (:`11`
            (`/Engine/EditorBlueprintResources/StandardMacros.FlipFlop`
              (:`A`
                (goto _label))
              (:`B`
                (goto _label_3))))
          (:`12`
            (`/Engine/EditorBlueprintResources/StandardMacros.FlipFlop`
              (:`A`
                (goto _label))
              (:`B`
                (goto _label_3)))))))))

(event `BPI_CheckComponent_1`
  (params (Component :type "SceneComponent Object Reference"))
  (if (`self.CanSetTarget`)
    (bind _output_get (set `self.TargetComponent` Component))
    (`|ExecutionSequence`
      (:`then_0`
        (for _array_element (`|MakeArray` (`self.box_5_pol_2`) (`self.box_4_pol_6`) (`self.box_4_pol_4`) (`self.box_4_pol_2`) (`self.box_6_pol_2`) (`self.box_4_pol_7`))
          (if (== _array_element _output_get)
            (set `self.RotationIndex` 1))))
      (:`then_1`
        (for _array_element_2 (`|MakeArray` (`self.box_4_pol_8`) (`self.box_4_pol_1`) (`self.box_4_pol_3`) (`self.box_4_pol_5`) (`self.box_1_typ_13`) (`self.box_6_pol_1`))
          (if (== _array_element_2 _output_get)
            (set `self.RotationIndex` 0))))
      (:`then_2`
        (if (== _output_get (`self.box_2_pol_2`))
          (set `self.RotationIndex` 2))))))

(fn `UserConstructionScript`)