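; Interactive wall unit whose individual door and panel pieces the player can open and close through interface calls.
; The component-check event stores the target piece and classifies it as one of three hinge rotations or a slide along relative Z.
; On interact, per-piece FlipFlops play or reverse one of two shared timelines that lerp rotation or location.
; Target changes are locked while a timeline plays.
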(event `self.ReceiveBeginPlay`
  (set `self.OriginalPosition0` (`SceneComponent.RelativeLocation` (`self.box_1_pol_3`)))
  (set `self.OriginalPosition1` (`SceneComponent.RelativeLocation` (`self.box_1_pol_1`)))
  (set `self.OriginalPosition2` (`SceneComponent.RelativeLocation` (`self.box_1_pol_2`))))

(event `/Game/BPI_PlayerInteraction.BPI_PlayerInteract`
  (bind _returnvalue (select `int` (`self.LocationIndex`) :`0` (`self.OriginalPosition0`) :`1` (`self.OriginalPosition1`) :`2` (`self.OriginalPosition2`)))
  (if (not (== (`self.TargetComponent`) (`self.Box`)))
    (switch `int` (`self.RotationIndex`)
      (:`0`
        (for (_array_element _array_index) (`|MakeArray` (`self.box_7_pol_5`) (`self.box_7_pol_2`) (`self.box_7_pol_3`) (`self.box_6_pol_3`) (`self.box_7_pol_4`) (`self.box_2_pol_1`)) :!label _label
          (if (== _array_element (`self.TargetComponent`))
            (switch `int` _array_index
              (:`0`
                (`/Engine/EditorBlueprintResources/StandardMacros.FlipFlop`
                  (:`A`
                    (set `self.CanSetTarget` false :!label _label_2)
                    (set `self.IsOpening` true)
                    (bind (_direction _newtrack_0) (`Timeline|Timeline` :!via `PlayFromStart` :!label _label_3)
                      (:`Update`
                        (`SceneComponent.K2_SetRelativeRotation` (`self.TargetComponent`) (`KismetMathLibrary.RLerp` (struct) (select `int` (`self.RotationIndex`) :`0` (struct :`Pitch` 90.0) :`1` (struct :`Pitch` -90.0) :`2` (struct :`Roll` 90.0) :!type "Rotator Structure") _newtrack_0) false false))
                      (:`Finished`
                        (set `self.CanSetTarget` true)
                        (set `self.IsOpening` false))))
                  (:`B`
                    (set `self.CanSetTarget` false :!label _label_4)
                    (set `self.IsOpening` true)
                    (goto _label_3 :!via `ReverseFromEnd`))))
              (:`1`
                (`/Engine/EditorBlueprintResources/StandardMacros.FlipFlop`
                  (:`A`
                    (goto _label_2))
                  (:`B`
                    (goto _label_4))))
              (:`2`
                (`/Engine/EditorBlueprintResources/StandardMacros.FlipFlop`
                  (:`A`
                    (goto _label_2))
                  (:`B`
                    (goto _label_4))))
              (:`3`
                (`/Engine/EditorBlueprintResources/StandardMacros.FlipFlop`
                  (:`A`
                    (goto _label_2))
                  (:`B`
                    (goto _label_4))))
              (:`4`
                (`/Engine/EditorBlueprintResources/StandardMacros.FlipFlop`
                  (:`A`
                    (goto _label_2))
                  (:`B`
                    (goto _label_4))))
              (:`5`
                (`/Engine/EditorBlueprintResources/StandardMacros.FlipFlop`
                  (:`A`
                    (goto _label_2))
                  (:`B`
                    (goto _label_4))))
              (:`6`
                (`/Engine/EditorBlueprintResources/StandardMacros.FlipFlop`
                  (:`A`
                    (goto _label_2))
                  (:`B`
                    (goto _label_4))))
              (:`7`
                (`/Engine/EditorBlueprintResources/StandardMacros.FlipFlop`
                  (:`A`
                    (goto _label_2))
                  (:`B`
                    (goto _label_4))))))))
      (:`1`
        (goto _label))
      (:`2`
        (goto _label))
      (:`3`
        (for (_array_element_2 _array_index_2) (`|MakeArray` (`self.box_1_pol_2`) (`self.box_1_pol_1`) (`self.box_1_pol_3`))
          (if (== _array_element_2 (`self.TargetComponent`))
            (switch `int` _array_index_2
              (:`0`
                (`/Engine/EditorBlueprintResources/StandardMacros.FlipFlop`
                  (:`A`
                    (set `self.CanSetTarget` false :!label _label_5)
                    (set `self.IsOpening` true)
                    (bind (_direction_2 _newtrack_0_2) (`Timeline|Timeline_0` :!via `PlayFromStart` :!label _label_6)
                      (:`Update`
                        (`SceneComponent.K2_SetRelativeLocation` (`self.TargetComponent`) (`KismetMathLibrary.VLerp` _returnvalue (`KismetMathLibrary.MakeVector` (.x _returnvalue) (.y _returnvalue) (+ (.z _returnvalue) 2.5)) _newtrack_0_2) false false))
                      (:`Finished`
                        (set `self.CanSetTarget` true)
                        (set `self.IsOpening` false))))
                  (:`B`
                    (set `self.CanSetTarget` false :!label _label_7)
                    (set `self.IsOpening` true)
                    (goto _label_6 :!via `ReverseFromEnd`))))
              (:`1`
                (`/Engine/EditorBlueprintResources/StandardMacros.FlipFlop`
                  (:`A`
                    (goto _label_5))
                  (:`B`
                    (goto _label_7))))
              (:`2`
                (`/Engine/EditorBlueprintResources/StandardMacros.FlipFlop`
                  (:`A`
                    (goto _label_5))
                  (:`B`
                    (goto _label_7)))))))))))

(event `/Game/BPI_PlayerInteraction.BPI_CheckComponent`
  (params (Component :type "SceneComponent Object Reference"))
  (if (`self.CanSetTarget`)
    (`self.F_SetTarget` Component)))

(fn `F_SetTarget`
  (params (TargetComponent :type "SceneComponent Object Reference"))
  (bind _output_get (set `self.TargetComponent` TargetComponent))
  (`|ExecutionSequence`
    (:`then_0`
      (for _array_element (`|MakeArray` (`self.box_7_pol_5`) (`self.box_6_pol_3`) (`self.box_7_pol_3`))
        (if (== _array_element _output_get)
          (set `self.RotationIndex` 0))))
    (:`then_1`
      (for _array_element_2 (`|MakeArray` (`self.box_7_pol_4`) (`self.box_7_pol_2`))
        (if (== _array_element_2 _output_get)
          (set `self.RotationIndex` 1))))
    (:`then_2`
      (if (== _output_get (`self.box_2_pol_1`))
        (set `self.RotationIndex` 2)))
    (:`then_3`
      (for (_array_element_3 _array_index) (`|MakeArray` (`self.box_1_pol_3`) (`self.box_1_pol_1`) (`self.box_1_pol_2`))
        (if (== _array_element_3 _output_get)
          (set `self.RotationIndex` 3)
          (set `self.LocationIndex` _array_index))))))

(fn `UserConstructionScript`)