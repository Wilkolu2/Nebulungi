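; BP_BaseDoors is a physics door the player can grab and swing with the mouse or push with a camera-directed impulse.
; Interface events handle key unlocking, impulse, and grab/release, which toggles player movement, look input and door input.
; While grabbed, mouse axes drive the door's yaw, with signs flipped by a dot-product check of the player's side.
; Overlapping the Lock component while not grabbed stops physics and marks the door closed.
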(event `/Game/BPI_PlayerInteraction.PBI_CheckKey`
  (set `self.IsLocked` false))

(event `/Game/BPI_PlayerInteraction.BPI_Impulse`
  (params (Camera :type "SceneComponent Object Reference"))
  (if (not (`self.IsLocked`))
    (`PrimitiveComponent.SetSimulatePhysics` (`self.Drzwi`) true)
    (`PrimitiveComponent.AddImpulse` (`self.Drzwi`) (* (`KismetMathLibrary.GetForwardVector` (`SceneComponent.K2_GetComponentRotation` Camera)) 750.0) "None" true)))

(event `/Game/BPI_PlayerInteraction.BPI_Grab`
  (params (PlayerCamre :type "CameraComponent Object Reference"))
  (bind _returnvalue (`GameplayStatics.GetPlayerController` 0))
  (set `self.IsGrabbed` true)
  (`CharacterMovementComponent.DisableMovement` (`Character.CharacterMovement` (`GameplayStatics.GetPlayerCharacter` 0)))
  (`Controller.SetIgnoreLookInput` _returnvalue true)
  (`self.EnableInput` _returnvalue)
  (if (not (`self.IsLocked`))
    (`PrimitiveComponent.SetSimulatePhysics` (`self.Drzwi`) true)))

(event `InputAxisKey|MouseY`
  (params (AxisValue :type "Float (single-precision)"))
  (bind _mouseinputmultiplier (`self.MouseInputMultiplier`))
  (bind (_returnvalue_roll _returnvalue_pitch _returnvalue_yaw) (`KismetMathLibrary.BreakRotator` (`SceneComponent.K2_GetComponentRotation` (`self.Drzwi`))))
  (bind (_returnvalue_roll_2 _returnvalue_pitch_2 _returnvalue_yaw_2) (`KismetMathLibrary.BreakRotator` (`SceneComponent.K2_GetComponentRotation` (`self.Arrow`))))
  (if (not (`self.IsLocked`)) :!label _label
    (`self.DoorMovement` (* (stale `InputAxisKey|MouseX` AxisValue) _mouseinputmultiplier) (* AxisValue _mouseinputmultiplier))
    (`SceneComponent.K2_SetWorldRotation` (`self.Arrow`) (`KismetMathLibrary.RInterpTo` (`SceneComponent.K2_GetComponentRotation` (stale `/Game/BPI_PlayerInteraction.BPI_Grab` PlayerCamre)) (`KismetMathLibrary.MakeRotator` _returnvalue_roll_2 _returnvalue_pitch_2 (+ _returnvalue_yaw_2 _returnvalue_yaw)) (stale `self.ReceiveTick` DeltaSeconds) 5.0) false false)))

(event `InputAxisKey|MouseX`
  (params (AxisValue :type "Float (single-precision)"))
  (goto _label))

(event `self.ReceiveTick`
  (params (DeltaSeconds :type "Float (single-precision)")))

(event `DoorMovement`
  (params (AmountX :type "Float (double-precision)") (AmountY :type "Float (double-precision)"))
  (bind _drzwi (`self.Drzwi`))
  (if (`self.IsGrabbed`)
    (`SceneComponent.K2_SetRelativeRotation` _drzwi (`KismetMathLibrary.ComposeRotators` (`SceneComponent.RelativeRotation` _drzwi) (`KismetMathLibrary.MakeRotator` 0.0 0.0 (/ (+ (* AmountX (select `bool` (>= (`KismetMathLibrary.Dot_VectorVector` (`KismetMathLibrary.Normal` (- (`self.K2_GetActorLocation` self) (`self.K2_GetActorLocation` (`GameplayStatics.GetPlayerCharacter` 0)))) (`self.GetActorForwardVector` self)) 0.0) :`false` 1.0 :`true` -1.0)) (* AmountY (select `bool` (>= (`KismetMathLibrary.Dot_VectorVector` (`KismetMathLibrary.Normal` (- (`self.K2_GetActorLocation` self) (`self.K2_GetActorLocation` (`GameplayStatics.GetPlayerCharacter` 0)))) (`self.GetActorForwardVector` self)) 0.0) :`false` -1.0 :`true` 1.0))) 2.0))) false false)
    (set `self.IsClosed` false)))

(event `/Game/BPI_PlayerInteraction.BPI_Release`
  (bind _returnvalue (`GameplayStatics.GetPlayerController` 0))
  (set `self.IsGrabbed` false)
  (`self.CheckIfOverlap`)
  (`KismetSystemLibrary.RetriggerableDelay` 0.2)
  (`CharacterMovementComponent.SetMovementMode` (`Character.CharacterMovement` (`GameplayStatics.GetPlayerCharacter` 0)) "MOVE_Walking" 0)
  (`self.DisableInput` _returnvalue)
  (`Controller.ResetIgnoreLookInput` _returnvalue))

(event `CheckIfOverlap`
  (for _array_element (`PrimitiveComponent.GetOverlappingComponents` (`self.Drzwi`))
    (if (== _array_element (`self.Lock`))
      (`self.CloseDoors`))))

(event `self.Lock.OnComponentBeginOverlap`
  (params (OverlappedComponent :type "PrimitiveComponent Object Reference") (OtherActor :type "Actor Object Reference") (OtherComp :type "PrimitiveComponent Object Reference") (OtherBodyIndex :type Integer) (bFromSweep :type Boolean) (SweepResult :type "HitResult Structure (by ref)"))
  (if (== OtherComp (`self.Drzwi`))
    (`self.CloseDoors`)))

(event `CloseDoors`
  (if (not (`self.IsGrabbed`))
    (set `self.IsClosed` true)
    (`PrimitiveComponent.SetSimulatePhysics` (`self.Drzwi`) false)))

(fn `UserConstructionScript`)