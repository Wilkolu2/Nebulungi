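; Interactive nightstand with two drawers that the player slides open and closed one at a time.
; An interface check records the targeted drawer, and player interaction toggles its own Timeline through a FlipFlop, lerping it along local X from its BeginPlay position.
; CheckTarget, IsOpening and per-drawer DoOnce gates lock targeting and input until movement finishes.
; The Construction Script snaps upper and lower content arrays to drawer sockets so items move with them.
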(event `self.ReceiveBeginPlay`
  (set `self.OriginalPosition0` (`SceneComponent.RelativeLocation` (`self.Szuflada0`)))
  (set `self.OriginalPosition1` (`SceneComponent.RelativeLocation` (`self.Szuflada1`))))

(event `/Game/BPI_PlayerInteraction.BPI_CheckComponent`
  (params (Component :type "SceneComponent Object Reference"))
  (if (`self.CheckTarget`)
    (set `self.TargetComponent` Component)))

(event `/Game/BPI_PlayerInteraction.BPI_PlayerInteract`
  (bind _originalposition0 (`self.OriginalPosition0`))
  (bind _originalposition1 (`self.OriginalPosition1`))
  (`|ExecutionSequence`
    (:`then_0`
      (if (== (`self.TargetComponent`) (`self.Szuflada0`))
        (if (not (`self.IsOpening`)) :!label _label
          (`|ExecutionSequence`
            (:`then_0`
              (if (== (`self.TargetComponent`) (`self.Szuflada0`))
                (`/Engine/EditorBlueprintResources/StandardMacros.DoOnce` false :!label _label_2
                  (:`Completed`
                    (set `self.CheckTarget` false)
                    (set `self.IsOpening` true)
                    (`/Engine/EditorBlueprintResources/StandardMacros.FlipFlop`
                      (:`A`
                        (bind (_direction _newtrack_0) (`Timeline|Timeline_3` :!label _label_3)
                          (:`Update`
                            (`SceneComponent.K2_SetRelativeLocation` (`self.TargetComponent`) (`KismetMathLibrary.VLerp` _originalposition0 (`KismetMathLibrary.MakeVector` 60.0 (.y _originalposition0) (.z _originalposition0)) _newtrack_0) false false))
                          (:`Finished`
                            (set `self.IsOpening` false)
                            (set `self.CheckTarget` true)
                            (set `self.TargetComponent` null)
                            (goto _label_2 :!via `Reset`))))
                      (:`B`
                        (goto _label_3 :!via `Reverse`)))))))
            (:`then_1`
              (if (== (`self.TargetComponent`) (`self.Szuflada1`))
                (`/Engine/EditorBlueprintResources/StandardMacros.DoOnce` false :!label _label_4
                  (:`Completed`
                    (set `self.CheckTarget` false)
                    (set `self.IsOpening` true)
                    (`/Engine/EditorBlueprintResources/StandardMacros.FlipFlop`
                      (:`A`
                        (bind (_direction_2 _newtrack_0_2) (`Timeline|Timeline_4` :!via `PlayFromStart` :!label _label_5)
                          (:`Update`
                            (`SceneComponent.K2_SetRelativeLocation` (`self.TargetComponent`) (`KismetMathLibrary.VLerp` _originalposition1 (`KismetMathLibrary.MakeVector` 60.0 (.y _originalposition1) (.z _originalposition1)) _newtrack_0_2) false false))
                          (:`Finished`
                            (set `self.IsOpening` false)
                            (set `self.CheckTarget` true)
                            (set `self.TargetComponent` null)
                            (goto _label_4 :!via `Reset`))))
                      (:`B`
                        (goto _label_5 :!via `Reverse`)))))))))))
    (:`then_1`
      (if (== (`self.TargetComponent`) (`self.Szuflada1`))
        (goto _label)))))

(fn `UserConstructionScript`
  (`|ExecutionSequence`
    (:`then_0`
      (for (_array_element _array_index) (`self.UpDrawerContent`)
        (`self.K2_AttachToComponent` _array_element (`self.Szuflada1`) (select `int` _array_index :`0` "Socket0" :`1` "Socket1" :`2` "Socket2" :!type "Name") "SnapToTarget" "KeepWorld" "KeepWorld" true)))
    (:`then_1`
      (for (_array_element_2 _array_index_2) (`self.DownDrawerContent`)
        (`self.K2_AttachToComponent` _array_element_2 (`self.Szuflada0`) (select `int` _array_index_2 :`0` "Socket0" :`1` "Socket1" :`2` "Socket2" :!type "Name") "SnapToTarget" "KeepWorld" "KeepWorld" true)))))