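; BP_ItemParent is the inventory system's base item actor, which a player can pick up through Blueprint interface events.
; Pickup checks the item's volume against a fixed inventory cap, sends ItemInfo and itself to the player, then destroys its mesh and stops ticking while the actor remains.
; Another event enables mesh physics; the impulse event is empty, with its camera-forward impulse node left disconnected.
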(event `/Game/BPI_PlayerInteraction.BPI_PickUpItem`
  (params (PlayerRef :type "Actor Object Reference") (Item :type "Actor Object Reference") (InventoryVolume :type Integer))
  (if (<= (+ InventoryVolume (`.ItemVolume_24_B96D065745EA1D3D652829B7E7E6BD9F` (break `/Game/KamilBlueprints/InventorySystem/S_ItemStruct` (`self.ItemInfo`)))) 10)
    (message `/Game/BPI_PlayerInteraction.BPI_AddToInventory` PlayerRef (`self.ItemInfo`) self)
    (`ActorComponent.K2_DestroyComponent` (`self.StaticMesh`))
    (`self.SetActorTickEnabled` false)))

(event `/Game/BPI_PlayerInteraction.BPI_Impulse`
  (params (Camera :type "SceneComponent Object Reference")))

(event `/Game/BPI_PlayerInteraction.BPI_SetSimulatePhysics`
  (`PrimitiveComponent.SetSimulatePhysics` (`self.StaticMesh`) true))

(fn `UserConstructionScript`)