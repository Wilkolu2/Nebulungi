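; Base interactable item that the player can pick up into their inventory.
; The Construction Script fills ItemInfo from DT_ItemInfo, using the ItemName enum as the row name.
; SeeText and UnseenText toggle the WhatToPress prompt and the CanIPickUp flag.
; Interact, when pickup is allowed and BP_Player's inventory has room, passes ItemInfo to the player's PickUp and destroys the actor.
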(event `/Game/Systems/BPI_InteractionSystem.Interact`
  (bind _player (`self.Player`))
  (bind _asbp_player (cast `/Game/FirstPerson/Blueprints/BP_Player` (`GameplayStatics.GetPlayerCharacter` 0)))
  (bind _output_get (set `self.Player` _asbp_player))
  (if (`self.CanIPickUp?`)
    (if (not (< (`/Game/FirstPerson/Blueprints/BP_Player.MaxEq` _player) (+ (`KismetArrayLibrary.Array_Length` (`/Game/FirstPerson/Blueprints/BP_Player.Inventory` _player)) 1)))
      (`/Game/FirstPerson/Blueprints/BP_Player.PickUp` _output_get (`self.ItemInfo`))
      (`self.K2_DestroyActor`))))

(event `SeeText`
  (`SceneComponent.SetVisibility` (`self.WhatToPress`) true false)
  (set `self.CanIPickUp?` true))

(event `UnseenText`
  (`SceneComponent.SetVisibility` (`self.WhatToPress`) false false)
  (set `self.CanIPickUp?` false))

(fn `UserConstructionScript`
  (bind _returnvalue (`|GetDataTableRow` "/Game/Game/Interactions/DT_ItemInfo.DT_ItemInfo" (`KismetStringLibrary.Conv_StringToName` (`|GetEnumeratorNameAsString` (`self.ItemName`))))
    (:`then`
      (set `self.ItemInfo` _returnvalue))))